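; BP_Collectable is a world item pickup that floats, falls, and gets pulled into the player's inventory.
; Tick applies simple gravity using a downward Visibility line trace, while timelines drive the mesh bob and a Launch vertical push.
; When BP_ThirdPersonCharacter stays inside CollecBubble through the spawn delay, the item homes toward them and calls ItemDataComponent.InteractWithMessage at close range.
; The construction script applies DataAsset material parameters to a dynamic MI_Block instance.
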(event `self.ReceiveBeginPlay`
  (`|ExecutionSequence`
    (:`then_0`
      (set `self.AbsorbDelay` (`self.SpawnDelay`)))
    (:`then_1`
      ;[1 1 1] Floating
      (bind (_direction _floatcurve) (`Timeline|Float` :!via `PlayFromStart`)
        (:`Update`
          (`SceneComponent.K2_SetRelativeLocation` (`self.StaticMesh`) (`KismetMathLibrary.MakeVector` -10.0 -10.0 (* _floatcurve (`self.floatRange`))) false false))))))

(event `self.CollecBubble.OnComponentBeginOverlap`
  (params (OverlappedComponent :type "PrimitiveComponent Object Reference") (OtherActor :type "Actor Object Reference") (OtherComp :type "PrimitiveComponent Object Reference") (OtherBodyIndex :type Integer) (bFromSweep :type Boolean) (SweepResult :type "HitResult Structure (by ref)"))
  ;[1 1 1] Overlap Check
  (bind _asbp_third_person_character (cast `/Game/ThirdPerson/Blueprints/BP_ThirdPersonCharacter` OtherActor))
  (set `self.Target Player` _asbp_third_person_character)
  (set `self.IsInRange` true))

(event `self.ReceiveTick`
  (params (DeltaSeconds :type "Float (single-precision)"))
  (bind _returnvalue (`self.K2_GetActorLocation`))
  ;[1 1 1] Simple Gravity
  (`|ExecutionSequence`
    (:`then_0`
      (if (and (`self.IsFalling`) (not (`self.IsAbsorbingNow`)))
        (set `self.GravityVelocity` (+ (`self.GravityVelocity`) (* (`self.GravityAccel`) DeltaSeconds)))
        (else
          (`/Engine/EditorBlueprintResources/StandardMacros.DoOnce` false :!label _label
            (:`Completed`
              (set `self.GravityVelocity` 0.0))))))
    (:`then_1`
      (bind (_outhit _returnvalue_2) (`KismetSystemLibrary.LineTraceSingle` :`Start` _returnvalue :`End` (+ _returnvalue (`KismetMathLibrary.MakeVector` 0.0 0.0 (`self.UnderRange`))) :`TraceChannel` "TraceTypeQuery1" :`DrawDebugType` "ForDuration"))
      (if _returnvalue_2
        (set `self.IsFalling` false)
        (else
          (set `self.IsFalling` true)
          (goto _label :!via `Reset`))))
    (:`then_2`
      (if (and (`self.IsFalling`) (not (`self.IsAbsorbingNow`)))
        (`self.K2_AddActorWorldOffset` (`KismetMathLibrary.MakeVector` 0.0 0.0 (* (`self.GravityVelocity`) -1.0)))))
    (:`then_3`
      ;[1 1 1] Absorb Item
      (if (or (`self.IsInRange`) (`self.IsAbsorbingNow`))
        (if (`self.IsAbsorbingNow`)
          (bind _target_player (`self.Target Player`)
            (:`then`
              (`self.K2_SetActorLocation` (+ (* (`GameplayStatics.GetWorldDeltaSeconds`) (`self.AbsorbSpeed`) (`KismetMathLibrary.Normal` (- (`self.K2_GetActorLocation` _target_player) (`self.K2_GetActorLocation`)))) (`self.K2_GetActorLocation`)))
              (if (< (`KismetMathLibrary.Vector_Distance` (`self.K2_GetActorLocation` (`self.Target Player`)) (`self.K2_GetActorLocation`)) 50.0)
                (message `/Game/Inventory/IInteractInterface.Interact With` (`self.ItemDataComponent`) (`self.Target Player`))))
            (:`else`
              (set `self.IsInRange` false)
              (set `self.IsAbsorbingNow` false)
              (set `self.AbsorbDelay` (`self.SpawnDelay`))
              (goto _label :!via `Reset`)))
          (else
            (bind _output_get (set `self.AbsorbDelay` (- (`self.AbsorbDelay`) DeltaSeconds)))
            (if (<= _output_get 0.0)
              (set `self.IsAbsorbingNow` true))))
        (else
          (set `self.AbsorbDelay` (`self.SpawnDelay`)))))))

(event `self.CollecBubble.OnComponentEndOverlap`
  (params (OverlappedComponent :type "PrimitiveComponent Object Reference") (OtherActor :type "Actor Object Reference") (OtherComp :type "PrimitiveComponent Object Reference") (OtherBodyIndex :type Integer))
  ;[1 1 1] Overlap Check
  (cast `/Game/ThirdPerson/Blueprints/BP_ThirdPersonCharacter` OtherActor)
  (if (not (`self.IsAbsorbingNow`))
    (set `self.Target Player` null))
  (set `self.IsInRange` false))

(event `Launch`
  ;[1 1 1] Launch
  (bind (_direction _power) (`Timeline|Launch Graph` :!via `PlayFromStart`)
    (:`Update`
      (`self.K2_AddActorWorldOffset` (`KismetMathLibrary.MakeVector` 0.0 0.0 (* _power (`self.LaunchPower`)))))))

(fn `UserConstructionScript`
  (bind _returnvalue (`PrimitiveComponent.CreateDynamicMaterialInstance` (`self.StaticMesh`) 0 "/Game/Yuchin/Materials/MI_Block.MI_Block" "None"))
  (`/Game/Yuchin/DataAssets/BaseClass/DA_Base.SetMaterialParameters` (`self.Data Asset`) _returnvalue))